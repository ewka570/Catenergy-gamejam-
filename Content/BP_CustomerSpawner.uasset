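; BP_CustomerSpawner is an actor that spawns BP_Customer actors into the game at the position and rotation of its CustomerSpawner component.
; BeginPlay spawns the first customer through a DoOnce gate.
; A SpawnCustomer custom event repeats the same spawn whenever it is called, with no cap or timer in this Blueprint.
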(event Custom|Spawn%20Customer
  (Game|SpawnActorfromClass "/Game/BP_Customer.BP_Customer_C" (Math|Transform|MakeTransform (Transformation|GetWorldLocation (Variables|Default|GetCustomerSpawner)) (Transformation|GetWorldRotation (Variables|Default|GetCustomerSpawner)) "1.000000,1.000000,1.000000") "Undefined" "MultiplyWithRoot" 0 0))

(event EventBeginPlay
  (Utilities|FlowControl|DoOnce false
    (:Completed
      (Game|SpawnActorfromClass "/Game/BP_Customer.BP_Customer_C" (Math|Transform|MakeTransform (Transformation|GetWorldLocation (Variables|Default|GetCustomerSpawner)) (Transformation|GetWorldRotation (Variables|Default|GetCustomerSpawner)) "1.000000,1.000000,1.000000") "Undefined" "MultiplyWithRoot" 0 0))))

(event Collision|EventActorBeginOverlap
  (params (OtherActor :type Actor%20Object%20Reference)))

(event EventTick
  (params (DeltaSeconds :type Float%20%28single-precision%29)))

(fn ConstructionScript)